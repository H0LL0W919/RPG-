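; Player stats component for BP_ThirdPersonCharacter that tracks health, stamina, XP and level.
; On BeginPlay it waits a tick, caches the owning character and initializes its HUD widget, which the stat functions then update directly.
; Health and stamina increases clamp to max, while decreases return whether the stat is depleted.
; Reaching max XP raises the level, increases the next threshold by a fixed amount and resets XP to zero, discarding overflow.
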(event EventBeginPlay
  (Utilities|FlowControl|DelayUntilNextTick)
  (bind _asbp_third_person_character (Utilities|Casting|CastToBP_ThirdPersonCharacter (Components|GetOwner)))
  (Variables|Default|SetplayerCharacterBP _asbp_third_person_character)
  (Progress|SetPercent (Variables|/Game/UI/PlayerHUD/WBP_Hud.WBP_Hud_C|GetStaminaBar (Variables|/Game/My_Blueprints/PlayerCharacter/BP_ThirdPersonCharacter.BP_ThirdPersonCharacter_C|GetHUD%20Widget (Variables|Default|GetplayerCharacterBP))) (/ (Variables|Stamina|GetcurrentStamina) (Variables|Stamina|GetmaxStamina)))
  (Progress|SetPercent (Variables|/Game/UI/PlayerHUD/WBP_Hud.WBP_Hud_C|GetHealthBar (Variables|/Game/My_Blueprints/PlayerCharacter/BP_ThirdPersonCharacter.BP_ThirdPersonCharacter_C|GetHUD%20Widget (Variables|Default|GetplayerCharacterBP))) (/ (Variables|Health|GetcurrentHealth) (Variables|Health|GetmaxHealth)))
  (Progress|SetPercent (Variables|/Game/UI/PlayerHUD/WBP_Hud.WBP_Hud_C|GetXPBar (Variables|/Game/My_Blueprints/PlayerCharacter/BP_ThirdPersonCharacter.BP_ThirdPersonCharacter_C|GetHUD%20Widget (Variables|Default|GetplayerCharacterBP))) (/ (Variables|Experience|GetXP) (Variables|Experience|GetmaxXP)))
  (Rendering|Components|TextRender|SetText (Variables|/Game/UI/PlayerHUD/WBP_Hud.WBP_Hud_C|GetXPText (Variables|/Game/My_Blueprints/PlayerCharacter/BP_ThirdPersonCharacter.BP_ThirdPersonCharacter_C|GetHUD%20Widget (Variables|Default|GetplayerCharacterBP))) (Utilities|Text|FormatText "{Current XP} / {Max XP}" (Variables|Experience|GetXP) (Variables|Experience|GetmaxXP)))
  (Rendering|Components|TextRender|SetText (Variables|/Game/UI/PlayerHUD/WBP_Hud.WBP_Hud_C|GetLevelText (Variables|/Game/My_Blueprints/PlayerCharacter/BP_ThirdPersonCharacter.BP_ThirdPersonCharacter_C|GetHUD%20Widget (Variables|Default|GetplayerCharacterBP))) (Utilities|Text|ToText(Integer) (Variables|Experience|Getlevel))))

(fn DecreaseCurrentHealth
  (params (Incoming%20Damage :type Float%20%28double-precision%29))
  (if (not (<= (Variables|Health|GetcurrentHealth) 0.0))
    (bind _output_get (Variables|Health|SetcurrentHealth (- (Variables|Health|GetcurrentHealth) Incoming%20Damage)))
    (Progress|SetPercent (Variables|/Game/UI/PlayerHUD/WBP_Hud.WBP_Hud_C|GetHealthBar (Variables|/Game/My_Blueprints/PlayerCharacter/BP_ThirdPersonCharacter.BP_ThirdPersonCharacter_C|GetHUD%20Widget (Variables|Default|GetplayerCharacterBP))) (/ _output_get (Variables|Health|GetmaxHealth)))
    (if (<= (Variables|Health|GetcurrentHealth) 0.0)
      _
      (else
        (return false))))
  (return true))

(fn IncreaseMaxHealth
  (params (Increase%20Max%20Health%20 :type Float%20%28double-precision%29))
  (Variables|Health|SetmaxHealth (+ (Variables|Health|GetmaxHealth) Increase%20Max%20Health%20))
  (Progress|SetPercent (Variables|/Game/UI/PlayerHUD/WBP_Hud.WBP_Hud_C|GetHealthBar (Variables|/Game/My_Blueprints/PlayerCharacter/BP_ThirdPersonCharacter.BP_ThirdPersonCharacter_C|GetHUD%20Widget (Variables|Default|GetplayerCharacterBP))) (/ (Variables|Health|GetcurrentHealth) (Variables|Health|GetmaxHealth))))

(fn DecreaseCurrentStamina
  (params (Stamina%20Decrease%20Amount :type Float%20%28double-precision%29))
  (if (not (<= (Variables|Stamina|GetcurrentStamina) 0.0))
    (Variables|Stamina|SetcurrentStamina (- (Variables|Stamina|GetcurrentStamina) Stamina%20Decrease%20Amount))
    (Progress|SetPercent (Variables|/Game/UI/PlayerHUD/WBP_Hud.WBP_Hud_C|GetStaminaBar (Variables|/Game/My_Blueprints/PlayerCharacter/BP_ThirdPersonCharacter.BP_ThirdPersonCharacter_C|GetHUD%20Widget (Variables|Default|GetplayerCharacterBP))) (/ (Variables|Stamina|GetcurrentStamina) (Variables|Stamina|GetmaxStamina)))
    (if (<= (Variables|Stamina|GetcurrentStamina) 0.0)
      _
      (else
        (return false))))
  (return true))

(fn IncreaseMaxStamina
  (params (Increase%20Max%20Stamina :type Float%20%28double-precision%29))
  (Variables|Stamina|SetmaxStamina (+ (Variables|Stamina|GetmaxStamina) Increase%20Max%20Stamina))
  (Progress|SetPercent (Variables|/Game/UI/PlayerHUD/WBP_Hud.WBP_Hud_C|GetStaminaBar (Variables|/Game/My_Blueprints/PlayerCharacter/BP_ThirdPersonCharacter.BP_ThirdPersonCharacter_C|GetHUD%20Widget (Variables|Default|GetplayerCharacterBP))) (/ (Variables|Stamina|GetcurrentStamina) (Variables|Stamina|GetmaxStamina))))

(fn IncreaseCurrentHealth
  (params (Increase%20Health :type Float%20%28double-precision%29))
  (Variables|Health|SetcurrentHealth (+ (Variables|Health|GetcurrentHealth) Increase%20Health))
  (if (> (Variables|Health|GetcurrentHealth) (Variables|Health|GetmaxHealth))
    (Variables|Health|SetcurrentHealth (Variables|Health|GetmaxHealth)))
  (Progress|SetPercent (Variables|/Game/UI/PlayerHUD/WBP_Hud.WBP_Hud_C|GetHealthBar (Variables|/Game/My_Blueprints/PlayerCharacter/BP_ThirdPersonCharacter.BP_ThirdPersonCharacter_C|GetHUD%20Widget (Variables|Default|GetplayerCharacterBP))) (/ (Variables|Health|GetcurrentHealth) (Variables|Health|GetmaxHealth))))

(fn IncreaseCurrentStamina
  (params (Increase%20Stamina :type Float%20%28double-precision%29))
  (Variables|Stamina|SetcurrentStamina (+ (Variables|Stamina|GetcurrentStamina) Increase%20Stamina))
  (if (> (Variables|Stamina|GetcurrentStamina) (Variables|Stamina|GetmaxStamina))
    (Variables|Stamina|SetcurrentStamina (Variables|Stamina|GetmaxStamina)))
  (Progress|SetPercent (Variables|/Game/UI/PlayerHUD/WBP_Hud.WBP_Hud_C|GetStaminaBar (Variables|/Game/My_Blueprints/PlayerCharacter/BP_ThirdPersonCharacter.BP_ThirdPersonCharacter_C|GetHUD%20Widget (Variables|Default|GetplayerCharacterBP))) (/ (Variables|Stamina|GetcurrentStamina) (Variables|Stamina|GetmaxStamina))))

(fn IncreaseXP
  (params (Increase%20Level :type Float%20%28double-precision%29))
  (Variables|Experience|SetXP (+ (Variables|Experience|GetXP) Increase%20Level))
  (if (>= (Variables|Experience|GetXP) (Variables|Experience|GetmaxXP))
    (Experience|IncreaseLevel 1))
  (Progress|SetPercent (Variables|/Game/UI/PlayerHUD/WBP_Hud.WBP_Hud_C|GetXPBar (Variables|/Game/My_Blueprints/PlayerCharacter/BP_ThirdPersonCharacter.BP_ThirdPersonCharacter_C|GetHUD%20Widget (Variables|Default|GetplayerCharacterBP))) (/ (Variables|Experience|GetXP) (Variables|Experience|GetmaxXP)))
  (Rendering|Components|TextRender|SetText (Variables|/Game/UI/PlayerHUD/WBP_Hud.WBP_Hud_C|GetXPText (Variables|/Game/My_Blueprints/PlayerCharacter/BP_ThirdPersonCharacter.BP_ThirdPersonCharacter_C|GetHUD%20Widget (Variables|Default|GetplayerCharacterBP))) (Utilities|Text|FormatText "{Current XP} / {Max XP}" (Variables|Experience|GetXP) (Variables|Experience|GetmaxXP))))

(fn IncreaseLevel
  (params (Added%20Level :type Integer))
  (Variables|Experience|Setlevel (+ (Variables|Experience|Getlevel) Added%20Level))
  (Variables|Experience|SetmaxXP (+ (Variables|Experience|GetmaxXP) 1.5e+02))
  (Variables|Experience|SetXP 0.0)
  (Rendering|Components|TextRender|SetText (Variables|/Game/UI/PlayerHUD/WBP_Hud.WBP_Hud_C|GetLevelText (Variables|/Game/My_Blueprints/PlayerCharacter/BP_ThirdPersonCharacter.BP_ThirdPersonCharacter_C|GetHUD%20Widget (Variables|Default|GetplayerCharacterBP))) (Utilities|Text|ToText(Integer) (Variables|Experience|Getlevel))))